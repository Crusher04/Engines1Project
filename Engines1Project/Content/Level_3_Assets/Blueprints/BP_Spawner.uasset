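; BP_Spawner is a Level 3 actor that spawns scaled-down BP_Ball actors at its own location and rotation.
; The first overlap spawns a ball once.
; Tick polls BallSpawned and EnableEventTick on the player's BP_ThirdPersonCharacter, clearing the latter before spawning another.
; After that spawn, it resets the character's BallsUsed and TotalScore once more than seven balls are used.
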(event `self.ReceiveActorBeginOverlap`
  (params (OtherActor :type "Actor Object Reference"))
  (`/Engine/EditorBlueprintResources/StandardMacros.DoOnce` false
    (:`Completed`
      (`self.Spawn Item`))))

(event `self.ReceiveTick`
  (params (DeltaSeconds :type "Float (single-precision)"))
  (bind _asbp_third_person_character (cast `/Game/ThirdPerson/Blueprints/BP_ThirdPersonCharacter` (`GameplayStatics.GetPlayerCharacter` 0)))
  (if (and (`/Game/ThirdPerson/Blueprints/BP_ThirdPersonCharacter.Ball Spawned` _asbp_third_person_character) (`/Game/ThirdPerson/Blueprints/BP_ThirdPersonCharacter.Enable event tick` _asbp_third_person_character))
    (set `/Game/ThirdPerson/Blueprints/BP_ThirdPersonCharacter.Enable event tick` false _asbp_third_person_character)
    (`self.Attempt To Spawn`)
    (`KismetSystemLibrary.Delay` 2.0)))

(fn `Attempt To Spawn`
  (bind _asbp_third_person_character (cast `/Game/ThirdPerson/Blueprints/BP_ThirdPersonCharacter` (`GameplayStatics.GetPlayerCharacter` 0)))
  (if (`/Game/ThirdPerson/Blueprints/BP_ThirdPersonCharacter.Ball Spawned` _asbp_third_person_character)
    (`self.Spawn Item`)
    (if (> (`/Game/ThirdPerson/Blueprints/BP_ThirdPersonCharacter.Balls Used` _asbp_third_person_character) 7)
      (set `/Game/ThirdPerson/Blueprints/BP_ThirdPersonCharacter.Balls Used` 0 _asbp_third_person_character)
      (set `/Game/ThirdPerson/Blueprints/BP_ThirdPersonCharacter.Total Score` 0 _asbp_third_person_character))))

(fn `Spawn Item`
  (bind (_returnvalue_x _returnvalue_y _returnvalue_z) (`KismetMathLibrary.BreakVector` (`self.K2_GetActorLocation`)))
  (bind _returnvalue (`|SpawnActorFromClass` "/Game/Level_3_Assets/Blueprints/BP_Ball.BP_Ball_C" (`KismetMathLibrary.MakeTransform` (`KismetMathLibrary.MakeVector` _returnvalue_x _returnvalue_y _returnvalue_z) (`self.K2_GetActorRotation`) (0.2 0.2 0.2)) "AdjustIfPossibleButAlwaysSpawn" "OverrideRootScale" null null))
  (set `self.Ball` _returnvalue))

(fn `UserConstructionScript`)