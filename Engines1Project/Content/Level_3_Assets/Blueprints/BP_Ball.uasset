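; BP_Ball is a skeeball that the player aims and tosses with E, using XValue for sideways position and YValue for projectile speed.
; Tick runs stepped X or Y slider functions depending on FindVelocity, though the Y slider only changes XValue, leaving YValue untouched.
; Hitting BP_Score increments the ball's PlayerScore.
; That hit or a four-second timeout destroys the ball and resets the third-person character's spawn flag and tick.
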(event `Key|E`
  (params (Key :type "Key Structure"))
  ;[1 1 1] Gets User Input to Aim & Toss Skeeball
  (:`Pressed`
    (`|ExecutionSequence`
      (:`then_0`
        (set `self.Find Velocity` true)
        (`SceneComponent.K2_SetWorldLocation` (`self.Sphere`) (`KismetMathLibrary.MakeVector` (`KismetMathLibrary.Conv_IntToDouble` (`self.X-Value`))) false false))
      (:`then_1`
        (set `ProjectileMovementComponent.InitialSpeed` (`KismetMathLibrary.Conv_IntToDouble` (`self.Y-Value`)) (`self.ProjectileMovement`))))))

(event `self.ReceiveTick`
  (params (DeltaSeconds :type "Float (single-precision)"))
  ;[1 1 1] Creates the Sliders to get Aim & Power
  (if (`self.Find Velocity`)
    (`self.Start Y Slider`)
    (else
      (`self.Start X Slider`))))

(event `self.Sphere.OnComponentHit`
  (params (HitComponent :type "PrimitiveComponent Object Reference") (OtherActor :type "Actor Object Reference") (OtherComp :type "PrimitiveComponent Object Reference") (NormalImpulse :type "Vector Structure") (Hit :type "HitResult Structure (by ref)"))
  (cast `/Game/Level_3_Assets/Blueprints/BP_Score` OtherActor)
  (set `self.Player Score` (+ (`self.Player Score`) 1))
  (`self.K2_DestroyActor`)
  (bind _asbp_third_person_character (cast `/Game/ThirdPerson/Blueprints/BP_ThirdPersonCharacter` (`GameplayStatics.GetPlayerCharacter` 0)))
  (set `/Game/ThirdPerson/Blueprints/BP_ThirdPersonCharacter.Ball Spawned` false _asbp_third_person_character)
  (set `/Game/ThirdPerson/Blueprints/BP_ThirdPersonCharacter.Enable event tick` true _asbp_third_person_character))

(event `self.ReceiveBeginPlay`
  (`KismetSystemLibrary.Delay` 4.0)
  (`/Engine/EditorBlueprintResources/StandardMacros.IsValid` (`self.Sphere`)
    (:`Is Valid`
      (`self.K2_DestroyActor`)
      (bind _asbp_third_person_character (cast `/Game/ThirdPerson/Blueprints/BP_ThirdPersonCharacter` (`GameplayStatics.GetPlayerCharacter` 0)))
      (set `/Game/ThirdPerson/Blueprints/BP_ThirdPersonCharacter.Ball Spawned` false _asbp_third_person_character)
      (set `/Game/ThirdPerson/Blueprints/BP_ThirdPersonCharacter.Enable event tick` true _asbp_third_person_character))))

(fn `Start X Slider`
  (`|ExecutionSequence`
    (:`then_0`
      (if (`self.X-NotMaxed`)
        (`KismetSystemLibrary.K2_SetTimer` null "" 0.2 true)
        (if (<= (`self.X-Value`) 0)
          (set `self.X-NotMaxed` false)
          (else
            (set `self.X-Value` (- (`self.X-Value`) 10))))
        (else
          (`KismetSystemLibrary.K2_SetTimer` null "" 0.2 true)
          (if (< (`self.X-Value`) (`self.X-Value Maxed`))
            (set `self.X-Value` (+ (`self.X-Value`) 10))))))))

(fn `Start Y Slider`
  (`|ExecutionSequence`
    (:`then_0`
      (if (`self.Y-NotMaxed`)
        (`KismetSystemLibrary.K2_SetTimer` null "" 0.2 true)
        (if (<= (`self.X-Value`) 0)
          (set `self.X-NotMaxed` false)
          (else
            (set `self.X-Value` (- (`self.X-Value`) 10))))
        (else
          (`KismetSystemLibrary.K2_SetTimer` null "" 0.2 true)
          (if (< (`self.X-Value`) (`self.X-Value Maxed`))
            (set `self.X-Value` (+ (`self.X-Value`) 10))))))))

(fn `UserConstructionScript`)