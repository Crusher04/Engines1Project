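; Saw pickup actor that gives the player the saw when its trigger is overlapped.
; Any overlap plays a sound, spawns a particle effect and destroys the actor, then sets IsSawPickedUp on the player character and shows a pickup message.
; The player reference used for the message is cached on BeginPlay.
; A timeline meant to spin the petrol cutter mesh is present but never started, so it does not run.
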(event `self.ReceiveBeginPlay`
  (bind _asbp_third_person_character (cast `/Game/ThirdPerson/Blueprints/BP_ThirdPersonCharacter` (`GameplayStatics.GetPlayerCharacter` 0)))
  (set `self.ThePlayer` _asbp_third_person_character))

(event `self.PickupTrigger.OnComponentBeginOverlap`
  (params (OverlappedComponent :type "PrimitiveComponent Object Reference") (OtherActor :type "Actor Object Reference") (OtherComp :type "PrimitiveComponent Object Reference") (OtherBodyIndex :type Integer) (bFromSweep :type Boolean) (SweepResult :type "HitResult Structure (by ref)"))
  (bind _returnvalue (`self.K2_GetActorLocation`))
  (`GameplayStatics.PlaySoundAtLocation` "/Game/UE5_RawAsset/Audio/Pickup.Pickup" _returnvalue (struct) 1.0 1.0 0.0 null null null null)
  (`GameplayStatics.SpawnEmitterAtLocation` "/Game/Realistic_Starter_VFX_Pack_Vol2/Particles/Hit/P_Ceramic.P_Ceramic" _returnvalue)
  (`self.K2_DestroyActor`)
  (bind _asbp_third_person_character (cast `/Game/ThirdPerson/Blueprints/BP_ThirdPersonCharacter` (`GameplayStatics.GetPlayerCharacter` 0)))
  (set `/Game/ThirdPerson/Blueprints/BP_ThirdPersonCharacter.IsSawPickedUp` true _asbp_third_person_character)
  (`/Game/ThirdPerson/Blueprints/BP_ThirdPersonCharacter.DisplayMessage` (`self.ThePlayer`) 3.0 "You Have Picked Up The Saw"))

(fn `UserConstructionScript`)